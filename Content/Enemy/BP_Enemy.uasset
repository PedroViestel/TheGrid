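; BP_Enemy is a shooter enemy that notices the player on capsule overlap or when hit, then turns to face them each tick.
; A DoOnce starts a looping timer that spawns projectiles from its Arrow; StopShooting clears it and ResetEnemies re-arms detection.
; Hits subtract health until the actor is destroyed.
; BeginPlay randomizes values for a vertical bobbing timeline, which nothing in the graph starts.
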(event `self.Capsule.OnComponentBeginOverlap`
  (params (OverlappedComponent :type "PrimitiveComponent Object Reference") (OtherActor :type "Actor Object Reference") (OtherComp :type "PrimitiveComponent Object Reference") (OtherBodyIndex :type Integer) (bFromSweep :type Boolean) (SweepResult :type "HitResult Structure (by ref)"))
  ;[1 1 1] Character noticy
  (set `self.IsCharNotice` true))

(event `self.ReceiveTick`
  (params (DeltaSeconds :type "Float (single-precision)"))
  ;[1 1 1] Look at character
  (if (`self.IsCharNotice`)
    (`|ExecutionSequence`
      (:`then_0`
        (`self.K2_SetActorRotation` (`KismetMathLibrary.FindLookAtRotation` (`self.K2_GetActorLocation`) (`self.K2_GetActorLocation` (`self.MainCharacter`)))))
      (:`then_1`
        (`/Engine/EditorBlueprintResources/StandardMacros.DoOnce` false :!label _label
          (:`Completed`
            (`KismetSystemLibrary.K2_SetTimer` null "Fire" (/ 1.0 (`self.BulletsPerSecond`)) true)))))))

(event `ResetEnemies`
  (set `self.IsCharNotice` false)
  (goto _label :!via `Reset`))

(event `StopShooting`
  (`KismetSystemLibrary.K2_ClearTimer` null "Fire"))

(event `self.ReceiveHit`
  (params (MyComp :type "PrimitiveComponent Object Reference") (Other :type "Actor Object Reference") (OtherComp :type "PrimitiveComponent Object Reference") (bSelfMoved :type Boolean) (HitLocation :type "Vector Structure") (HitNormal :type "Vector Structure") (NormalImpulse :type "Vector Structure") (Hit :type "HitResult Structure (by ref)"))
  (bind _health (`self.Health`))
  ;[1 1 1] Hit
  (set `self.Health` (- _health 10))
  (`KismetSystemLibrary.PrintString` (`KismetStringLibrary.Conv_IntToString` _health))
  (set `self.IsCharNotice` true)
  (if (<= _health 0)
    (`self.K2_DestroyActor`)))

(event `self.ReceiveBeginPlay`
  (bind _returnvalue (`self.K2_GetActorLocation`))
  (`|ExecutionSequence`
    (:`then_0`
      ;[1 1 1] Enemy Animation
      (set `self.StartLocation` _returnvalue)
      (set `self.EndLocation` (+ _returnvalue (`KismetMathLibrary.MakeVector` 0.0 0.0 (`KismetMathLibrary.RandomFloatInRange` 50.0 100.0))))
      (`TimelineComponent.SetPlayRate` (`self.EnemyLoop`) (`KismetMathLibrary.RandomFloatInRange` 1.0 2.0)))
    (:`then_1`
      (bind _asbp_character (cast `/Game/HeroChar/BP_Character` (`GameplayStatics.GetPlayerCharacter` 0)))
      (set `self.MainCharacter` _asbp_character))))

(fn `Fire`
  (`|SpawnActorFromClass` "/Game/Enemy/BP_ProjectileEnemy.BP_ProjectileEnemy_C" (`SceneComponent.K2_GetComponentToWorld` (`self.Arrow`)) "Undefined" "OverrideRootScale" null null))

(fn `UserConstructionScript`)
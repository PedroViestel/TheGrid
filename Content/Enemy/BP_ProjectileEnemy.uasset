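; BP_ProjectileEnemy is an enemy projectile that damages the player character on impact.
; On BeginPlay it sets a short lifespan and caches the player's BP_Character as Hero.
; Its Hit event calls DamageReceived on Hero with DamageDealed when the struck actor is that player, then destroys the projectile whatever it hit.
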(event `self.ReceiveBeginPlay`
  (`self.SetLifeSpan` 3.0)
  (bind _asbp_character (cast `/Game/HeroChar/BP_Character` (`GameplayStatics.GetPlayerCharacter` 0)))
  (set `self.Hero` _asbp_character))

(event `self.ReceiveHit`
  (params (MyComp :type "PrimitiveComponent Object Reference") (Other :type "Actor Object Reference") (OtherComp :type "PrimitiveComponent Object Reference") (bSelfMoved :type Boolean) (HitLocation :type "Vector Structure") (HitNormal :type "Vector Structure") (NormalImpulse :type "Vector Structure") (Hit :type "HitResult Structure (by ref)"))
  (bind _hero (`self.Hero`))
  (if (== Other _hero)
    (`/Game/HeroChar/BP_Character.DamageReceived` _hero (`self.DamageDealed`)))
  (`self.K2_DestroyActor`))

(fn `UserConstructionScript`)
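; Gameplay game mode that sets up the player HUD and handles the hero's death.
; On BeginPlay it caches the player character, adds the HUD widget to the viewport and binds to the character's HeroDied dispatcher.
; UpdateUI copies current health into the HUD text and progress bar.
; On death it hides the character and weapon, possesses the first checkpoint actor found and stops all enemies shooting.
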(event `Update UI`
  (bind _hudref (`self.HUDRef`))
  (bind _currenthealth (`/Game/HeroChar/BP_Character.CurrentHealth` (`self.MainCharacter`)))
  (set `/Game/HUD/HUDPlayer.HealthText` (`KismetTextLibrary.Conv_DoubleToText` _currenthealth "HalfToEven") _hudref)
  (if (> _currenthealth 0.0)
    (set `/Game/HUD/HUDPlayer.ProgressBarValue` (/ _currenthealth 100.0) _hudref)
    (else
      (set `/Game/HUD/HUDPlayer.ProgressBarValue` 0.0 _hudref))))

(event `self.ReceiveBeginPlay`
  (`|ExecutionSequence`
    (:`then_0`
      (bind _asbp_character (cast `/Game/HeroChar/BP_Character` (`GameplayStatics.GetPlayerCharacter` 0)))
      (set `self.MainCharacter` _asbp_character))
    (:`then_1`
      (bind _returnvalue (`|CreateWidget` "/Game/HUD/HUDPlayer.HUDPlayer_C" (`GameplayStatics.GetPlayerController` 0)))
      (bind _output_get (set `self.HUDRef` _returnvalue))
      (`UserWidget.AddToViewport` _output_get 0))
    (:`then_2`
      ;[1 1 1] Hero Died
      (add `/Game/HeroChar/BP_Character.HeroDied` (`self.MainCharacter`) (delegate `HeroDiedEvent`)))))

(event `HeroDiedEvent`
  ;[1 1 1] Hero Died
  (`self.HideMainCharacter`)
  (`self.PossessCheckPoint`)
  (`self.StopAllEnemies`))

(fn `HideMainCharacter`
  (bind _maincharacter (`self.MainCharacter`))
  (`self.SetActorHiddenInGame` _maincharacter true)
  (`self.SetActorHiddenInGame` (`/Game/HeroChar/BP_Character.Weapon` _maincharacter) true))

(fn `PossessCheckPoint`
  (bind _outactors (`GameplayStatics.GetAllActorsOfClass` "/Game/CheckPoint/BP_CheckPoint.BP_CheckPoint_C"))
  (`Controller.Possess` (`GameplayStatics.GetPlayerController` 0) (`|GetArrayItem` _outactors)))

(fn `StopAllEnemies`
  (bind _outactors (`GameplayStatics.GetAllActorsOfClass` "/Game/Enemy/BP_Enemy.BP_Enemy_C"))
  (for _array_element _outactors
    (`/Game/Enemy/BP_Enemy.StopShooting` _array_element)))

(fn `UserConstructionScript`)
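; BP_Totem is a red, blue or green totem that activates on Interact when the game mode reports the player has the matching key.
; Activation plays a timeline that slides TotemExternal, brightens the glow material and spawns a BP_KeyFake at the Arrow, tinted to the totem's color.
; The construction script creates the dynamic glow material; key flags are only read, and nothing blocks repeat activation.
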(event `/Game/Totem/BI_Interactable.Interact`
  (bind _gamemoderef (`self.GameModeref`))
  ;[1 1 1] Add Key to Totem
  (switch `/Game/Key/EnumKeys` (`self.TotemType`)
    (:`NewEnumerator0`
      (if (`/Game/Gamelogic/BP_GameplayGameMode.HasRedKey` _gamemoderef)
        (`TimelineComponent.PlayFromStart` (`self.TotemAnimation`))
        (`MaterialInstanceDynamic.SetScalarParameterValue` (`self.TotemMaterial`) "Emissive" (`self.EmissiveWhenActivated`))
        (bind _returnvalue (`self.SpawnFakeKey`))
        (`self.SetKeyColor` _returnvalue (struct :`R` 1.0 :`A` 1.0))))
    (:`NewEnumerator1`
      (if (`/Game/Gamelogic/BP_GameplayGameMode.HasBlueKey` _gamemoderef)
        (`TimelineComponent.PlayFromStart` (`self.TotemAnimation`))
        (`MaterialInstanceDynamic.SetScalarParameterValue` (`self.TotemMaterial`) "Emissive" (`self.EmissiveWhenActivated`))
        (bind _returnvalue_2 (`self.SpawnFakeKey`))
        (`self.SetKeyColor` _returnvalue_2 (struct :`B` 1.0 :`A` 1.0))))
    (:`NewEnumerator2`
      (if (`/Game/Gamelogic/BP_GameplayGameMode.HasGreenKey` _gamemoderef)
        (`TimelineComponent.PlayFromStart` (`self.TotemAnimation`))
        (`MaterialInstanceDynamic.SetScalarParameterValue` (`self.TotemMaterial`) "Emissive" (`self.EmissiveWhenActivated`))
        (bind _returnvalue_3 (`self.SpawnFakeKey`))
        (`self.SetKeyColor` _returnvalue_3 (struct :`G` 1.0 :`A` 1.0))))))

(event `self.ReceiveBeginPlay`
  ;[1 1 1] Get Game Mode Ref
  (bind _asbp_gameplay_game_mode (cast `/Game/Gamelogic/BP_GameplayGameMode` (`GameplayStatics.GetGameMode`)))
  (set `self.GameModeref` _asbp_gameplay_game_mode))

(fn `SetKeyColor`
  (params (Key :type "/Game/Key/BP_KeyFake Object Reference") (Color :type "LinearColor Structure"))
  (bind _returnvalue (`PrimitiveComponent.CreateDynamicMaterialInstance` (`/Game/Key/BP_KeyFake.Frame1` Key) 0 "/Game/Material/M_Glow.M_Glow" "None"))
  (`MaterialInstanceDynamic.SetVectorParameterValue` _returnvalue "BaseColor" Color)
  (`MaterialInstanceDynamic.SetScalarParameterValue` _returnvalue "Emissive" 20.0)
  (bind _returnvalue_2 (`PrimitiveComponent.CreateDynamicMaterialInstance` (`/Game/Key/BP_KeyFake.Frame2` Key) 0 "/Game/Material/M_Glow.M_Glow" "None"))
  (`MaterialInstanceDynamic.SetVectorParameterValue` _returnvalue_2 "BaseColor" Color)
  (`MaterialInstanceDynamic.SetScalarParameterValue` _returnvalue_2 "Emissive" 20.0))

(fn `SpawnFakeKey`
  (returns (ReturnValue :type "/Game/Key/BP_KeyFake Object Reference"))
  (bind _returnvalue (`|SpawnActorFromClass` "/Game/Key/BP_KeyFake.BP_KeyFake_C" (`SceneComponent.K2_GetComponentToWorld` (`self.Arrow`)) "Undefined" "OverrideRootScale" null null))
  (return _returnvalue))

(fn `UserConstructionScript`
  (bind _returnvalue (`PrimitiveComponent.CreateDynamicMaterialInstance` (`self.TotemBase`) 1 "/Game/Material/M_Glow.M_Glow" "None"))
  (bind _output_get (set `self.TotemMaterial` _returnvalue))
  (`MaterialInstanceDynamic.SetScalarParameterValue` _output_get "Emissive" (`self.Emissive`))
  (`MaterialInstanceDynamic.SetVectorParameterValue` _output_get "BaseColor" (`self.BaseColor`)))
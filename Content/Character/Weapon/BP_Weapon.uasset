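; BP_Weapon is an automatic weapon that spawns BP_Projectile actors for the player character.
; StartShooting fires immediately, then repeats FireWeapon on a looping timer paced by BulletsPerSecond until StopShooting clears it.
; Each shot spawns at the ProjectilePosition transform on player 0's BP_Character, cached at BeginPlay, rather than at a point on the weapon itself.
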(event `StartShooting`
  (`self.FireWeapon`)
  (`KismetSystemLibrary.K2_SetTimer` null "FireWeapon" (/ 1.0 (`self.BulletsPerSecond`)) true))

(event `StopShooting`
  (`KismetSystemLibrary.K2_ClearTimer` null "FireWeapon"))

(event `self.ReceiveBeginPlay`
  (bind _asbp_character (cast `/Game/Character/BP_Character` (`GameplayStatics.GetPlayerCharacter` 0)))
  (set `self.Player` _asbp_character))

(fn `FireWeapon`
  (`|SpawnActorFromClass` "/Game/Character/Weapon/BP_Projectile.BP_Projectile_C" (`SceneComponent.K2_GetComponentToWorld` (`/Game/Character/BP_Character.ProjectilePosition` (`self.Player`))) "Undefined" "OverrideRootScale" null null))

(fn `UserConstructionScript`)
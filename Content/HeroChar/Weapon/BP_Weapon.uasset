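; BP_Weapon is the hero character's automatic weapon, firing BP_Projectile actors while shooting is active.
; StartShooting fires once immediately, then runs a looping timer on FireWeapon at a rate set by BulletsPerSecond; StopShooting clears it.
; BeginPlay caches player 0 as BP_Character, whose ProjectilePosition component supplies each projectile's spawn transform.
; Each shot also prints a "Fire" debug message.
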(event `StartShooting`
  (`self.FireWeapon`)
  (`KismetSystemLibrary.K2_SetTimer` null "FireWeapon" (/ 1.0 (`self.BulletsPerSecond`)) true))

(event `StopShooting`
  (`KismetSystemLibrary.K2_ClearTimer` null "FireWeapon"))

(event `self.ReceiveBeginPlay`
  (bind _asbp_character (cast `/Game/HeroChar/BP_Character` (`GameplayStatics.GetPlayerCharacter` 0)))
  (set `self.Player` _asbp_character))

(fn `FireWeapon`
  (`|SpawnActorFromClass` "/Game/HeroChar/Weapon/BP_Projectile.BP_Projectile_C" (`SceneComponent.K2_GetComponentToWorld` (`/Game/HeroChar/BP_Character.ProjectilePosition` (`self.Player`))) "Undefined" "OverrideRootScale" null null)
  (`KismetSystemLibrary.PrintString` "Fire" true true (struct :`G` 0.66 :`B` 1.0 :`A` 1.0) 15.0))

(fn `UserConstructionScript`)